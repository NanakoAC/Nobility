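; Player character Blueprint that handles weapon cycling and the response to death.
; It calls CycleWeapon on BeginPlay and from mouse wheel input, where a small Boolean macro turns the up or down entry into a true or false argument for one shared call.
; When the Health component fires OnDied, Ragdoll runs only with authority; a DestroyActor node is left unconnected.
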(event `self.ReceiveBeginPlay`
  (`self.CycleWeapon` false))

(event `Key|MouseScrollUp`
  (params (Key :type "Key Structure"))
  (:`Pressed`
    (bind _returnvalue (`self.Boolean` :!label _label))
    (`self.CycleWeapon` _returnvalue)))

(event `Key|MouseScrollDown`
  (params (Key :type "Key Structure"))
  (:`Pressed`
    (goto _label :!via `execute2`)))

(event `self.Health.OnDied`
  (if (`self.HasAuthority`)
    (`self.Ragdoll`)))

(fn `UserConstructionScript`)